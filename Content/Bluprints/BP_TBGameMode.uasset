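; BP_TBGameMode is a game mode that tracks progress, remaining time and the number of working enemy characters.
; BeginPlay seeds the worker count from all BP_EnemyCharacter actors and starts a looping one-second timer.
; Each timer call increments progress, adjusts the count by comparing each enemy's IsWorking and WasWorking flags, and prints it.
; Tick lowers remaining time by a fixed step each frame, independent of delta time.
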(event `self.ReceiveBeginPlay`
  (`KismetSystemLibrary.K2_SetTimer` null "Progress increase" 1.0 true)
  (bind _outactors (`GameplayStatics.GetAllActorsOfClass` "/Game/Bluprints/BP_EnemyCharacter.BP_EnemyCharacter_C"))
  (set `self.StartAmountOfWorkers` (`KismetArrayLibrary.Array_Length` _outactors)))

(event `Progress increase`
  (set `self.CurrentProgress` (+ (`self.CurrentProgress`) 1.0))
  (bind _outactors (`GameplayStatics.GetAllActorsOfClass` "/Game/Bluprints/BP_EnemyCharacter.BP_EnemyCharacter_C"))
  (for _array_element _outactors
    (if (`/Game/Bluprints/BP_EnemyCharacter.IsWorking` _array_element)
      (bind _wasworking (`/Game/Bluprints/BP_EnemyCharacter.WasWorking` _array_element))
      (if (not _wasworking)
        (set `self.StartAmountOfWorkers` (+ (`self.StartAmountOfWorkers`) 1)))
      (elif _wasworking
        (set `self.StartAmountOfWorkers` (- (`self.StartAmountOfWorkers`) 1)))))
  (`KismetSystemLibrary.PrintString` (`KismetStringLibrary.Conv_IntToString` (`self.StartAmountOfWorkers`))))

(event `self.ReceiveTick`
  (params (DeltaSeconds :type "Float (single-precision)"))
  (set `self.RemainingTime` (- (`self.RemainingTime`) 0.1)))

(fn `UserConstructionScript`)