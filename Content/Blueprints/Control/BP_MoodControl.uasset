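; BP_MoodControl is an interaction point that sends the player character on a timed move to a mood point.
; Its Box overlap adds a W_Interact widget to the viewport and removes it when the overlap ends.
; IncreaseMood, if the ThirdPersonCharacter can execute orders, sets its move flag and blocks further orders.
; After the character's stat-increase delay, it clears the move flag and re-enables orders.
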(event `self.Box.OnComponentBeginOverlap`
  (params (OverlappedComponent :type "PrimitiveComponent Object Reference") (OtherActor :type "Actor Object Reference") (OtherComp :type "PrimitiveComponent Object Reference") (OtherBodyIndex :type Integer) (bFromSweep :type Boolean) (SweepResult :type "HitResult Structure (by ref)"))
  (bind _returnvalue (`|CreateWidget` "/Game/UI/W_Interact.W_Interact_C"))
  (`UserWidget.AddToViewport` _returnvalue 0))

(event `self.Box.OnComponentEndOverlap`
  (params (OverlappedComponent :type "PrimitiveComponent Object Reference") (OtherActor :type "Actor Object Reference") (OtherComp :type "PrimitiveComponent Object Reference") (OtherBodyIndex :type Integer))
  (bind _foundwidgets (`WidgetBlueprintLibrary.GetAllWidgetsOfClass` "/Game/UI/W_Interact.W_Interact_C"))
  (`Widget.RemoveFromParent` _foundwidgets))

(event `/Game/Blueprints/Interfaces/BPI_MoodPoint.Increase Mood`
  ;[1 1 1] Activates AI movement
  (bind _asthird_person_character (cast `/Game/Blueprints/Characters/ThirdPersonCharacter` (`GameplayStatics.GetPlayerCharacter` 0)))
  (if (`/Game/Blueprints/Characters/ThirdPersonCharacter.CanExecuteOrders` _asthird_person_character)
    (set `TBCharacter.MoveToMoodPoint` true _asthird_person_character)
    (set `/Game/Blueprints/Characters/ThirdPersonCharacter.CanExecuteOrders` false _asthird_person_character)
    (`KismetSystemLibrary.Delay` (`/Game/Blueprints/Characters/ThirdPersonCharacter.DelayForStatIncrease` _asthird_person_character))
    (set `TBCharacter.MoveToMoodPoint` false _asthird_person_character)
    (set `/Game/Blueprints/Characters/ThirdPersonCharacter.CanExecuteOrders` true _asthird_person_character)))

(fn `UserConstructionScript`)