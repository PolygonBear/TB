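; BP_TBGameMode is a game mode that tracks a progress counter tied to the player's Table, alongside a RemainingTime countdown.
; ToggleProgress starts or clears a looping one-second timer; the progress event increments and prints CurrentProgress while the ThirdPersonCharacter's Table is valid.
; RemainingTime drops by a fixed step every Tick, so its rate follows frame rate.
; StopTimer and TableEvent are stubs, and an EventGraph timer setup is unconnected.
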(event `self.ReceiveTick`
  (params (DeltaSeconds :type "Float (single-precision)"))
  (set `self.RemainingTime` (- (`self.RemainingTime`) 0.1)))

(event `Progress increase`
  (bind _asthird_person_character (cast `/Game/ThirdPersonCPP/Blueprints/ThirdPersonCharacter` (`GameplayStatics.GetPlayerCharacter` 0)))
  (`/Engine/EditorBlueprintResources/StandardMacros.IsValid` (`/Game/ThirdPersonCPP/Blueprints/ThirdPersonCharacter.Table` _asthird_person_character)
    (:`Is Valid`
      (bind _output_get (set `self.CurrentProgress` (+ (`self.CurrentProgress`) 1.0)))
      (`KismetSystemLibrary.PrintString` (`KismetStringLibrary.Conv_DoubleToString` _output_get)))))

(fn `StopTimer`)

(fn `TableEvent`
  (returns (IsNearTheTable :type Boolean))
  (return false))

(fn `ToggleProgress`
  (bind _handle (`self.Handle`))
  (if (`KismetSystemLibrary.K2_IsTimerActiveHandle` _handle)
    (`KismetSystemLibrary.K2_ClearAndInvalidateTimerHandle` _handle)
    (else
      (bind _returnvalue (`KismetSystemLibrary.K2_SetTimerDelegate` (`|CreateDelegate` :!event `Progress increase`) 1.0 true))
      (set `self.Handle` _returnvalue))))

(fn `UserConstructionScript`)