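; BP_TBGameInstance is a Game Instance Blueprint that provides events for showing the game's main menu, credits, options and pause screens.
; Each event lazily creates its widget the first time, caches it in a variable, and adds it to the viewport, reusing that instance on later calls.
; Only the options widget is created with an explicit owning player, the first player controller.
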(event `ShowMainMenu`
  (`/Engine/EditorBlueprintResources/StandardMacros.IsValid` (`self.WD_MainMenu`)
    (:`Is Valid`
      _)
    (:`Is Not Valid`
      (bind _returnvalue (`|CreateWidget` "/Game/UI/Menu/W_MainMenu.W_MainMenu_C"))
      (bind _output_get (set `self.WD_MainMenu` _returnvalue))))
  (`UserWidget.AddToViewport` _output_get 0))

(event `ShowCredits`
  (`/Engine/EditorBlueprintResources/StandardMacros.IsValid` (`self.WD_Credits`)
    (:`Is Valid`
      _)
    (:`Is Not Valid`
      (bind _returnvalue (`|CreateWidget` "/Game/UI/Menu/W_Credits.W_Credits_C"))
      (bind _output_get (set `self.WD_Credits` _returnvalue))))
  (`UserWidget.AddToViewport` _output_get 0))

(event `ShowOptions`
  (`/Engine/EditorBlueprintResources/StandardMacros.IsValid` (`self.WD_Options`)
    (:`Is Valid`
      _)
    (:`Is Not Valid`
      (bind _returnvalue (`|CreateWidget` "/Game/UI/Menu/W_Options.W_Options_C" (`GameplayStatics.GetPlayerController` 0)))
      (bind _output_get (set `self.WD_Options` _returnvalue))))
  (`UserWidget.AddToViewport` _output_get 0))

(event `ShowGamePause`
  (`/Engine/EditorBlueprintResources/StandardMacros.IsValid` (`self.WD_GamePause`)
    (:`Is Valid`
      _)
    (:`Is Not Valid`
      (bind _returnvalue (`|CreateWidget` "/Game/UI/Menu/W_Pause.W_Pause_C"))
      (bind _output_get (set `self.WD_GamePause` _returnvalue))))
  (`UserWidget.AddToViewport` _output_get 0))