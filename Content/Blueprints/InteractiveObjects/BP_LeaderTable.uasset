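; BP_LeaderTable is an interactable table that toggles a progress state or display through BP_TBGameMode when the user interacts.
; Its Box overlap shows a W_Interact prompt for any actor and registers the table on an overlapping ThirdPersonCharacter.
; Ending overlap removes top-level W_Interact widgets and clears that character's Table reference.
; UserInteracted calls ToggleProgress on the game mode, while TableEvent simply returns false.
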(event `self.Box.OnComponentBeginOverlap`
  (params (OverlappedComponent :type "PrimitiveComponent Object Reference") (OtherActor :type "Actor Object Reference") (OtherComp :type "PrimitiveComponent Object Reference") (OtherBodyIndex :type Integer) (bFromSweep :type Boolean) (SweepResult :type "HitResult Structure (by ref)"))
  (bind _returnvalue (`|CreateWidget` "/Game/UI/W_Interact.W_Interact_C"))
  (`UserWidget.AddToViewport` _returnvalue 0)
  (bind _asthird_person_character (cast `/Game/Blueprints/Characters/ThirdPersonCharacter` OtherActor))
  (set `/Game/Blueprints/Characters/ThirdPersonCharacter.Table` self _asthird_person_character))

(event `self.Box.OnComponentEndOverlap`
  (params (OverlappedComponent :type "PrimitiveComponent Object Reference") (OtherActor :type "Actor Object Reference") (OtherComp :type "PrimitiveComponent Object Reference") (OtherBodyIndex :type Integer))
  (bind _foundwidgets (`WidgetBlueprintLibrary.GetAllWidgetsOfClass` "/Game/UI/W_Interact.W_Interact_C"))
  (`Widget.RemoveFromParent` _foundwidgets)
  (bind _asthird_person_character (cast `/Game/Blueprints/Characters/ThirdPersonCharacter` OtherActor))
  (set `/Game/Blueprints/Characters/ThirdPersonCharacter.Table` null _asthird_person_character))

(fn `TableEvent`
  (returns (IsNearTheTable :type Boolean))
  (return false))

(fn `UserConstructionScript`)

(fn `UserInteracted`
  (bind _asbp_tbgame_mode (cast `/Game/Blueprints/Characters/BP_TBGameMode` (`GameplayStatics.GetGameMode`)))
  (`/Game/Blueprints/Characters/BP_TBGameMode.ToggleProgress` _asbp_tbgame_mode))