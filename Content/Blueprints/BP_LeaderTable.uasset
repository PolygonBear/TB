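; BP_LeaderTable is an interactable table that raises the game's progress while something overlaps its Box.
; Begin overlap shows a W_Interact widget, sets IsNearTheTable on the player's ThirdPersonCharacter and starts a looping one-second timer that increments CurrentProgress in BP_TBGameMode.
; End overlap removes the widget, resets the flag and clears the timer by setting its time to zero.
; Neither overlap event checks which actor triggered it.
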(event `self.Box.OnComponentBeginOverlap`
  (params (OverlappedComponent :type "PrimitiveComponent Object Reference") (OtherActor :type "Actor Object Reference") (OtherComp :type "PrimitiveComponent Object Reference") (OtherBodyIndex :type Integer) (bFromSweep :type Boolean) (SweepResult :type "HitResult Structure (by ref)"))
  (bind _returnvalue (`|CreateWidget` "/Game/UI/W_Interact.W_Interact_C"))
  (`UserWidget.AddToViewport` _returnvalue 0)
  (bind _asthird_person_character (cast `/Game/ThirdPersonCPP/Blueprints/ThirdPersonCharacter` (`GameplayStatics.GetPlayerCharacter` 0)))
  (set `/Game/ThirdPersonCPP/Blueprints/ThirdPersonCharacter.IsNearTheTable` true _asthird_person_character)
  (`KismetSystemLibrary.K2_SetTimer` null "Progress increase" 1.0 true))

(event `self.Box.OnComponentEndOverlap`
  (params (OverlappedComponent :type "PrimitiveComponent Object Reference") (OtherActor :type "Actor Object Reference") (OtherComp :type "PrimitiveComponent Object Reference") (OtherBodyIndex :type Integer))
  (bind _foundwidgets (`WidgetBlueprintLibrary.GetAllWidgetsOfClass` "/Game/UI/W_Interact.W_Interact_C"))
  (`Widget.RemoveFromParent` _foundwidgets)
  (bind _asthird_person_character (cast `/Game/ThirdPersonCPP/Blueprints/ThirdPersonCharacter` (`GameplayStatics.GetPlayerCharacter` 0)))
  (set `/Game/ThirdPersonCPP/Blueprints/ThirdPersonCharacter.IsNearTheTable` false _asthird_person_character)
  (`KismetSystemLibrary.K2_SetTimer` null "Progress increase" 0.0 true))

(event `Progress increase`
  (bind _asbp_tbgame_mode (cast `/Game/Blueprints/BP_TBGameMode` (`GameplayStatics.GetGameMode`)))
  (set `/Game/Blueprints/BP_TBGameMode.CurrentProgress` (+ (`/Game/Blueprints/BP_TBGameMode.CurrentProgress` _asbp_tbgame_mode) 1.0) _asbp_tbgame_mode))

(fn `UserConstructionScript`)